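; Battery pickup actor that gives the player a battery when touched.
; On overlap with its Battery component, it casts the player pawn to VRPawn and calls AddBattery, or falls back to ThirdPersonCharacter, incrementing and printing its Batteries count.
; The pickup destroys itself after either grant, and also when the referenced SingleEnemy touches it, without granting anything.
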(event `self.Battery.OnComponentBeginOverlap`
  (params (OverlappedComponent :type "PrimitiveComponent Object Reference") (OtherActor :type "Actor Object Reference") (OtherComp :type "PrimitiveComponent Object Reference") (OtherBodyIndex :type Integer) (bFromSweep :type Boolean) (SweepResult :type "HitResult Structure (by ref)"))
  (if (== OtherActor (`GameplayStatics.GetPlayerPawn` 0))
    (bind _asvrpawn (cast `/Game/VRTemplate/Blueprints/VRPawn` OtherActor)
      (:`then`
        (`/Game/VRTemplate/Blueprints/VRPawn.AddBattery` _asvrpawn)
        (`self.K2_DestroyActor` :!label _label))
      (:`CastFailed`
        (bind _asthird_person_character (cast `/Game/TP/ThirdPersonBP/Blueprints/ThirdPersonCharacter` OtherActor)
          (:`then`
            (bind _output_get (set `/Game/TP/ThirdPersonBP/Blueprints/ThirdPersonCharacter.batteries` (+ (`/Game/TP/ThirdPersonBP/Blueprints/ThirdPersonCharacter.batteries` _asthird_person_character) 1) _asthird_person_character))
            (`KismetSystemLibrary.PrintString` (`KismetStringLibrary.Conv_IntToString` _output_get))
            (goto _label))
          (:`CastFailed`
            (`KismetSystemLibrary.PrintString` "Invalid player")))))
    (elif (== OtherActor "/Game/Blueprints/SingleEnemy.SingleEnemy")
      (goto _label))))

(fn `UserConstructionScript`)