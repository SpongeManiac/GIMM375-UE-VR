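; VR selection component that tracks hover and select states and reports them through event dispatchers.
; Hover and select enter and exit events set the state flags and broadcast each change.
; Releasing a selection while still hovered also fires the Execute dispatcher, while leaving hover mid-selection ends the selection without executing, giving button-style click-and-cancel behavior.
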(event `HoverEnter`
  (bind _output_get (set `self.Hover` true))
  (`self.HoverDispatcher` _output_get))

(event `HoverExit`
  (bind _output_get (set `self.Hover` false))
  (`self.HoverDispatcher` _output_get)
  (if (`self.Selecting`)
    (`self.SelectExit`)))

(event `SelectEnter`
  (bind _output_get (set `self.Selecting` true))
  (`self.SelectDispatcher` _output_get))

(event `SelectExit`
  (bind _output_get (set `self.Selecting` false))
  (`self.SelectDispatcher` _output_get)
  (if (`self.Hover`)
    (`self.ExecuteDispatcher`)))