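; LootSpawner is an actor that conditionally spawns a loot item through its LootLocation child actor component.
; SpawnLoot rolls a 0–1 value from the supplied random stream and, if it is at most Rarity, sets the child actor class to Loot and returns true.
; A debug print shows a roll and Rarity, but its roll is evaluated separately from the one compared.
; The event graph and construction script are empty.
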(fn `SpawnLoot`
  (params (StreamIn :type "RandomStream Structure (by ref)"))
  (returns (Success :type Boolean))
  (locals (LevelSeed :type "RandomStream Structure"))
  (bind _rarity (`self.Rarity`))
  (bind _returnvalue (/ (`KismetMathLibrary.Conv_IntToDouble` (`KismetMathLibrary.RandomIntegerFromStream` 1000 StreamIn)) 1000.0))
  (`KismetSystemLibrary.PrintString` (`KismetStringLibrary.Concat_StrStr` "Got " (`KismetStringLibrary.Conv_DoubleToString` _returnvalue) ", Rarity is " (`KismetStringLibrary.Conv_DoubleToString` _rarity)))
  (if (<= _returnvalue _rarity)
    (`ChildActorComponent.SetChildActorClass` (`self.LootLocation`) (`self.Loot`))
    (return true)
    (else
      (return false))))

(fn `UserConstructionScript`)