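; Enemy actor that wanders aimlessly until it detects a "Powered" actor (a battery), then pursues it.
; BeginPlay randomizes a redirection interval and loops a Delay to pick new wander directions.
; Tick steps one unit per frame toward the target or wander direction, sweeping only while wandering; MoveSpeed is unused.
; BatteryDetection overlaps toggle pursuit; HurtTrigger only reassigns the target, as its damage logic is disconnected.
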(event `self.ReceiveTick`
  (params (DeltaSeconds :type "Float (single-precision)"))
  (bind _returnvalue (`self.K2_GetActorLocation`))
  (bind _returnvalue_2 (`self.K2_GetActorLocation`))
  (bind _returnvalue_3 (`self.K2_GetActorLocation` (`self.batteryTarget`)))
  (bind _returnvalue_4 (+ _returnvalue (`self.randomDirection`)))
  (if (`self.batteryDetected`)
    ;[1 1 1] Move towards the battery.
    (`self.K2_SetActorTransform` (`KismetMathLibrary.MakeTransform` (+ (`KismetMathLibrary.GetDirectionUnitVector` _returnvalue_2 _returnvalue_3) _returnvalue_2) (`KismetMathLibrary.RInterpTo` (`KismetMathLibrary.Conv_VectorToRotator` _returnvalue_2) (`KismetMathLibrary.MakeRotator` (.roll (`KismetMathLibrary.FindLookAtRotation` _returnvalue_2 _returnvalue_3)) (.pitch (`KismetMathLibrary.FindLookAtRotation` _returnvalue_2 _returnvalue_3)) (.yaw (`KismetMathLibrary.FindLookAtRotation` _returnvalue_2 _returnvalue_3))) (`GameplayStatics.GetWorldDeltaSeconds`))))
    (else
      ;[1 1 1] Move in random directions aimlessly
      (`self.K2_SetActorTransform` (`KismetMathLibrary.MakeTransform` (+ (`KismetMathLibrary.GetDirectionUnitVector` _returnvalue _returnvalue_4) _returnvalue) (`KismetMathLibrary.RInterpTo` (`KismetMathLibrary.Conv_VectorToRotator` _returnvalue) (`KismetMathLibrary.MakeRotator` (.roll (`KismetMathLibrary.FindLookAtRotation` _returnvalue _returnvalue_4)) (.pitch (`KismetMathLibrary.FindLookAtRotation` _returnvalue _returnvalue_4)) (.yaw (`KismetMathLibrary.FindLookAtRotation` _returnvalue _returnvalue_4))) (`GameplayStatics.GetWorldDeltaSeconds`))) true))))

(event `self.ReceiveBeginPlay`
  ;[1 1 1] Set all traits to random at the start of the game.
  (set `self.moveSpeed` (* (+ (`KismetMathLibrary.RandomFloat`) 1.0) 5.0)) ; Movement speed. Unimplemented
  (set `self.newRandomDirectionSpeed` (* (+ (`KismetMathLibrary.RandomFloat`) 0.2) 2.0)) ; The rate at which the enemy picks a new direction to wander
  (set `self.randomDirection` (`KismetMathLibrary.RandomUnitVector`) :!label _label) ; Picks a new direction to wander. Looped based on newrandomdirectionspeed.
  (`KismetSystemLibrary.Delay` (`self.newRandomDirectionSpeed`))
  (goto _label))

(event `self.BatteryDetection.OnComponentBeginOverlap`
  (params (OverlappedComponent :type "PrimitiveComponent Object Reference") (OtherActor :type "Actor Object Reference") (OtherComp :type "PrimitiveComponent Object Reference") (OtherBodyIndex :type Integer) (bFromSweep :type Boolean) (SweepResult :type "HitResult Structure (by ref)"))
  ;[1 1 1] Look for powered objects. If they are nearby, check "Battery Detected" to pursue them. If I lose sight of powered objects, uncheck it.
  (if (`self.batteryDetected`)
    _
    (elif (`self.ActorHasTag` OtherActor "Powered")
      (set `self.batteryTarget` OtherActor)
      (set `self.batteryDetected` true))))

(event `self.BatteryDetection.OnComponentEndOverlap`
  (params (OverlappedComponent :type "PrimitiveComponent Object Reference") (OtherActor :type "Actor Object Reference") (OtherComp :type "PrimitiveComponent Object Reference") (OtherBodyIndex :type Integer))
  ;[1 1 1] Look for powered objects. If they are nearby, check "Battery Detected" to pursue them. If I lose sight of powered objects, uncheck it.
  (if (`self.ActorHasTag` OtherActor "Powered")
    (set `self.batteryDetected` false)))

(event `self.HurtTrigger.OnComponentBeginOverlap`
  (params (OverlappedComponent :type "PrimitiveComponent Object Reference") (OtherActor :type "Actor Object Reference") (OtherComp :type "PrimitiveComponent Object Reference") (OtherBodyIndex :type Integer) (bFromSweep :type Boolean) (SweepResult :type "HitResult Structure (by ref)"))
  (if true
    (set `self.batteryTarget` OtherActor)))

(fn `UserConstructionScript`)