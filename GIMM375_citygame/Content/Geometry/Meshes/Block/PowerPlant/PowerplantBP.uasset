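; Power plant actor where the player deposits batteries into five slots, winning once five are placed.
; Each slot's box overlap calls EvaluateDeposit, which takes a battery from the player's ThirdPersonCharacter_DoNotUse, applies the battery material and collision to the box's parent mesh, and destroys the box.
; CheckWin then triggers the character's Win or prints a remaining-battery message with a fixed count.
; The VRPawn branch is empty, so VR players cannot deposit.
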(event `self.Deposit5.OnComponentBeginOverlap`
  (params (OverlappedComponent :type "PrimitiveComponent Object Reference") (OtherActor :type "Actor Object Reference") (OtherComp :type "PrimitiveComponent Object Reference") (OtherBodyIndex :type Integer) (bFromSweep :type Boolean) (SweepResult :type "HitResult Structure (by ref)"))
  (bind _asbox_collision (cast `BoxComponent` OverlappedComponent))
  (`self.EvaluateDeposit` _asbox_collision OtherActor))

(event `self.Deposit1.OnComponentBeginOverlap`
  (params (OverlappedComponent :type "PrimitiveComponent Object Reference") (OtherActor :type "Actor Object Reference") (OtherComp :type "PrimitiveComponent Object Reference") (OtherBodyIndex :type Integer) (bFromSweep :type Boolean) (SweepResult :type "HitResult Structure (by ref)"))
  (bind _asbox_collision (cast `BoxComponent` OverlappedComponent))
  (`self.EvaluateDeposit` _asbox_collision OtherActor))

(event `self.Deposit2.OnComponentBeginOverlap`
  (params (OverlappedComponent :type "PrimitiveComponent Object Reference") (OtherActor :type "Actor Object Reference") (OtherComp :type "PrimitiveComponent Object Reference") (OtherBodyIndex :type Integer) (bFromSweep :type Boolean) (SweepResult :type "HitResult Structure (by ref)"))
  (bind _asbox_collision (cast `BoxComponent` OverlappedComponent))
  (`self.EvaluateDeposit` _asbox_collision OtherActor))

(event `self.Deposit3.OnComponentBeginOverlap`
  (params (OverlappedComponent :type "PrimitiveComponent Object Reference") (OtherActor :type "Actor Object Reference") (OtherComp :type "PrimitiveComponent Object Reference") (OtherBodyIndex :type Integer) (bFromSweep :type Boolean) (SweepResult :type "HitResult Structure (by ref)"))
  (bind _asbox_collision (cast `BoxComponent` OverlappedComponent))
  (`self.EvaluateDeposit` _asbox_collision OtherActor))

(event `self.Deposit4.OnComponentBeginOverlap`
  (params (OverlappedComponent :type "PrimitiveComponent Object Reference") (OtherActor :type "Actor Object Reference") (OtherComp :type "PrimitiveComponent Object Reference") (OtherBodyIndex :type Integer) (bFromSweep :type Boolean) (SweepResult :type "HitResult Structure (by ref)"))
  (bind _asbox_collision (cast `BoxComponent` OverlappedComponent))
  (`self.EvaluateDeposit` _asbox_collision OtherActor))

(fn `ActivateBattery`
  (params (BatteryMesh :type "StaticMeshComponent Object Reference"))
  (`PrimitiveComponent.SetMaterial` BatteryMesh 0 "/Game/Materials/Battery.Battery")
  (`PrimitiveComponent.SetCollisionEnabled` BatteryMesh "QueryAndPhysics"))

(fn `CheckWin`
  (returns (Won :type Boolean))
  (return (>= (`self.batteries`) 5)))

(fn `EvaluateDeposit`
  (params (DepositCollision :type "BoxComponent Object Reference") (ActorCollided :type "Actor Object Reference"))
  (bind _gotplayer (`self.Is Player` ActorCollided))
  (if _gotplayer
    (cast `/Game/VRTemplate/Blueprints/VRPawn` ActorCollided
      (:`CastFailed`
        (bind _asthird_person_character_do_not_use (cast `/Game/TP/ThirdPersonBP/Blueprints/ThirdPersonCharacter_Current` ActorCollided)
          (:`then`
            (if (>= (`/Game/TP/ThirdPersonBP/Blueprints/ThirdPersonCharacter_Current.batteries` _asthird_person_character_do_not_use) 1)
              (`/Engine/EditorBlueprintResources/StandardMacros.IncrementInt` (`self.batteries`)
                (:`  `
                  (`/Game/TP/ThirdPersonBP/Blueprints/ThirdPersonCharacter_Current.SubtractBattery` _asthird_person_character_do_not_use)
                  (`/Engine/EditorBlueprintResources/StandardMacros.DoOnce` false
                    (:`Completed`
                      (bind _asstatic_mesh_component (cast `StaticMeshComponent` (`|GetArrayItem` (`SceneComponent.GetParentComponents` DepositCollision))))
                      (`self.ActivateBattery` _asstatic_mesh_component)
                      (`ActorComponent.K2_DestroyComponent` DepositCollision)
                      (bind _won (`self.CheckWin`))
                      (if _won
                        (`/Game/TP/ThirdPersonBP/Blueprints/ThirdPersonCharacter_Current.Win` _asthird_person_character_do_not_use)
                        (else
                          (`KismetSystemLibrary.PrintString` (`KismetStringLibrary.Concat_StrStr` "You need " (`KismetStringLibrary.Conv_IntToString` (- 5 1)) " more battery(s)."))))))))))
          (:`CastFailed`
            (`KismetSystemLibrary.PrintString` "Invalid Player")))))))

(fn `Is Player`
  (params (Player :type "Actor Object Reference"))
  (returns (GotPlayer :type Boolean))
  (bind _output_get (set `self.actor` Player))
  (return (== _output_get (`GameplayStatics.GetPlayerPawn` 0))))

(fn `UserConstructionScript`)