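; HouseBP is a residential house Blueprint that hosts battery loot spawners.
; On BeginPlay it spawns a BatterySpawner at the world location of each ChildActorComponent, stores it in LootSpawners and attaches it to the house with KeepRelative rules.
; CreateLoot passes a Stream to SpawnLoot on every stored spawner.
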(event `self.ReceiveBeginPlay`
  (for _array_element (`self.K2_GetComponentsByClass` "/Script/Engine.ChildActorComponent")
    (bind _returnvalue (`|SpawnActorFromClass` "/Game/Blueprints/BatterySpawner.BatterySpawner_C" (`KismetMathLibrary.MakeTransform` (`SceneComponent.K2_GetComponentLocation` _array_element)) "Undefined" "OverrideRootScale" null null))
    (`KismetArrayLibrary.Array_Add` (`self.LootSpawners`) _returnvalue)
    (`self.K2_AttachToActor` _returnvalue self "None" "KeepRelative" "KeepRelative" "KeepRelative" true)))

(fn `CreateLoot`
  (params (Stream :type "RandomStream Structure"))
  (for _array_element (`self.LootSpawners`)
    (`/Game/Blueprints/LootSpawner.SpawnLoot` _array_element Stream)))

(fn `UserConstructionScript`)