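; DowntownBP is a downtown block actor that exposes the spawners of its houses and can spawn a single enemy.
; GetSpawners casts each child actor to HouseBP and appends that house's spawners to its own Spawners array, which it returns without clearing first.
; SpawnEnemy rolls the LevelSeed random stream against EnemyRarity and, on success, always spawns SingleEnemy at the EnemySpawner component's location.
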(event `self.ReceiveBeginPlay`)

(fn `GetSpawners`
  (returns (LootSpawners :type "Array of /Game/Blueprints/Loot/LootSpawner Object Reference"))
  (locals (LevelSeed :type "RandomStream Structure"))
  (for _array_element (`self.K2_GetComponentsByClass` "/Script/Engine.ChildActorComponent")
    (bind _ashouse_bp (cast `/Game/Geometry/Meshes/Block/Residential/HouseBP` (`ChildActorComponent.ChildActor` _array_element)))
    (bind _spawners (`/Game/Geometry/Meshes/Block/Residential/HouseBP.Get Spawners` _ashouse_bp))
    (`KismetArrayLibrary.Array_Append` (`self.Spawners`) _spawners))
  (return (`self.Spawners`)))

(fn `SpawnEnemy`
  (params (LevelSeed :type "RandomStream Structure (by ref)"))
  (if (<= (`KismetMathLibrary.RandomFloatInRangeFromStream` 0.0 1.0 LevelSeed) (`self.enemyRarity`))
    (`|SpawnActorFromClass` "/Game/Blueprints/SingleEnemy.SingleEnemy_C" (`KismetMathLibrary.MakeTransform` (`SceneComponent.K2_GetComponentLocation` (`self.EnemySpawner`))) "AlwaysSpawn" "OverrideRootScale" null null)))

(fn `UserConstructionScript`)