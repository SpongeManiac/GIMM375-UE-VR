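; Boid actor, an early prototype that is meant to turn toward the player pawn each tick, with no flocking logic.
; Tick feeds RInterpTo a rotation derived from the actor's location vector and a look-at target with yaw zeroed.
; The interpolation has no delta time or speed supplied, so the look-at target does not take effect.
; A zero-vector AddForce follows, so no thrust is applied.
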(event `self.ReceiveBeginPlay`)

(event `self.ReceiveTick`
  (params (DeltaSeconds :type "Float (single-precision)"))
  (bind _returnvalue (`self.K2_GetActorLocation`))
  (`self.K2_SetActorRotation` (`KismetMathLibrary.RInterpTo` (`KismetMathLibrary.Conv_VectorToRotator` _returnvalue) (`KismetMathLibrary.MakeRotator` (.roll (`KismetMathLibrary.FindLookAtRotation` _returnvalue (`self.K2_GetActorLocation` (`GameplayStatics.GetPlayerPawn` 0)))) (.pitch (`KismetMathLibrary.FindLookAtRotation` _returnvalue (`self.K2_GetActorLocation` (`GameplayStatics.GetPlayerPawn` 0)))))))
  (`PrimitiveComponent.AddForce` (0.0 0.0 0.0)))

(fn `UserConstructionScript`)