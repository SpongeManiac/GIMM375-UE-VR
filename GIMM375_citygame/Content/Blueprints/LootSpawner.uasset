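; LootSpawner is a Blueprint that randomly spawns a Loot actor, with Rarity as the chance threshold.
; SpawnLoot takes a random stream, rolls a normalized value and, if it is at or below Rarity, spawns Loot at LootLocation and attaches it to itself.
; A debug print shows Rarity and a roll, drawn separately from the one compared.
; The event graph and construction script are empty.
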(fn `SpawnLoot`
  (params (Stream :type "RandomStream Structure"))
  (bind _rarity (`self.Rarity`))
  (bind _returnvalue (/ (`KismetMathLibrary.Conv_IntToDouble` (`KismetMathLibrary.RandomIntegerFromStream` 1000 Stream)) 1000.0))
  (`KismetSystemLibrary.PrintString` (`KismetStringLibrary.Concat_StrStr` "Got " (`KismetStringLibrary.Conv_DoubleToString` _returnvalue) ", Rarity is " (`KismetStringLibrary.Conv_DoubleToString` _rarity)))
  (if (<= _returnvalue _rarity)
    (bind _returnvalue_2 (`|SpawnActorFromClass` (`self.Loot`) (`KismetMathLibrary.MakeTransform` (`SceneComponent.K2_GetComponentLocation` (`self.LootLocation`))) "Undefined" "OverrideRootScale" null null))
    (`self.K2_AttachToActor` _returnvalue_2 self "None" "KeepRelative" "KeepRelative" "KeepRelative" true)))

(fn `UserConstructionScript`)