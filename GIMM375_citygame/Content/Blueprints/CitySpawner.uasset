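; CitySpawner procedurally builds a city grid on BeginPlay, tiling a repeating pattern of intersections, roads and city blocks.
; CreateCity positions tiles using their width and height, stores them by grid coordinate and attaches them to a CityOffset actor.
; PostCreate then shifts that offset by a corner-derived center, populates one random block as powerplant and others as residential, and applies final scale.
; A clock-seeded stream drives most random choices, though residential variants use unseeded RandomInteger.
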(event `self.ReceiveBeginPlay`
  (`self.CreateCity` (`|MakeMap` 1 (make `/Game/Geometry/Meshes/Roads/Pattern` (`|MakeMap` 1 "/Game/Geometry/Meshes/Roads/Intersection_Blueprint.Intersection_Blueprint_C" 0 "/Game/Geometry/Meshes/Roads/Road_H_Blueprint.Road_H_Blueprint_C" :!valuetype "/Game/Geometry/Meshes/Roads/BaseRoad Class Reference")) 0 (make `/Game/Geometry/Meshes/Roads/Pattern` (`|MakeMap` 1 "/Game/Geometry/Meshes/Roads/Road_V_Blueprint.Road_V_Blueprint_C" 0 "/Game/Geometry/Meshes/Roads/CityBlock_Blueprint.CityBlock_Blueprint_C" :!valuetype "/Game/Geometry/Meshes/Roads/BaseRoad Class Reference"))) (make `/Game/Geometry/Meshes/Roads/Vector2Int` (`self.Height`) (`self.Width`))))

(fn `CreateCity`
  (params (ActorPattern :type "Map of Integer to /Game/Geometry/Meshes/Roads/Pattern Structure") (Size :type "/Game/Geometry/Meshes/Roads/Vector2Int Structure"))
  (locals (Row :type Integer) (Column :type Integer) (Pattern :type String) (PatternPos :type Integer))
  (bind _returnvalue (`self.GetTransform`))
  (bind _returnvalue_2 (`self.GetTransform`))
  (bind _city (`self.City`))
  (bind _row (`local.Row`))
  (bind _current (`self.Current`))
  (bind (_x _y) (break `/Game/Geometry/Meshes/Roads/Vector2Int` (`self.PatternSize`)))
  (bind (_x_2 _y_2) (break `/Game/Geometry/Meshes/Roads/Vector2Int` (`self.Size`)))
  (bind _vector2int (make `/Game/Geometry/Meshes/Roads/Vector2Int` (`local.Row`) (`local.Column`)))
  (bind (_value _returnvalue_3) (`BlueprintMapLibrary.Map_Find` (`self.Patterns`) (mod _row _y)))
  (`self.GenerateSeed`)
  (bind _returnvalue_4 (`|SpawnActorFromClass` "/Game/Blueprints/CityOffset.CityOffset_C" (`KismetMathLibrary.MakeTransform` (`KismetMathLibrary.MakeVector` (.x (.location _returnvalue_2)) (.y (.location _returnvalue_2)) (.z (.location _returnvalue_2)))) "Undefined" "OverrideRootScale" null null))
  (`self.K2_AttachToActor` _returnvalue_4 self "None" "KeepWorld" "KeepRelative" "KeepRelative" false)
  (set `self.CityOffset` _returnvalue_4)
  (set `self.Size` Size)
  (bind _output_get (set `self.Patterns` ActorPattern))
  (bind (_value_2 _returnvalue_5) (`BlueprintMapLibrary.Map_Find` _output_get))
  (if _returnvalue_5
    (set `self.PatternSize` (make `/Game/Geometry/Meshes/Roads/Vector2Int` (`BlueprintMapLibrary.Map_Length` (`.Objects_5_4484C8884B4986133814AD9ACAD7955D` (break `/Game/Geometry/Meshes/Roads/Pattern` _value_2))) (`BlueprintMapLibrary.Map_Length` _output_get)))
    (set `self.ObjectPos` (.location (`self.GetTransform`)))
    (for _index (range 1 (+ _y_2 1))
      (set `local.Row` _index)
      (for _index_2 (range 1 (+ _x_2 1))
        (bind _output_get_2 (set `local.Column` _index_2))
        (if _returnvalue_3
          (bind (_value_3 _returnvalue_6) (`BlueprintMapLibrary.Map_Find` (`.Objects_5_4484C8884B4986133814AD9ACAD7955D` (break `/Game/Geometry/Meshes/Roads/Pattern` _value)) (mod _output_get_2 _x)))
          (if _returnvalue_6
            (bind _returnvalue_7 (`|SpawnActorFromClass` _value_3 (`KismetMathLibrary.MakeTransform` (`self.ObjectPos`)) "Undefined" "OverrideRootScale" null null))
            (`self.K2_AttachToActor` _returnvalue_7 (`self.CityOffset`) "None" "KeepRelative" "KeepWorld" "KeepRelative" true)
            (bind _output_get_3 (set `self.Current` _returnvalue_7))
            (if (and (== _output_get_2 1) (!= _row 1))
              (bind _height (`/Game/Geometry/Meshes/Roads/BaseRoad.GetHeight` _output_get_3))
              (bind _output_get_4 (set `self.ObjectPos` (+ (`self.ObjectPos`) (`KismetMathLibrary.MakeVector` (`KismetMathLibrary.Conv_IntToDouble` _height)))))
              (`SceneComponent.K2_SetWorldTransform` (`/Game/Geometry/Meshes/Roads/BaseRoad.DefaultSceneRoot` _output_get_3) (`KismetMathLibrary.MakeTransform` _output_get_4) false false))
            (`BlueprintMapLibrary.Map_Remove` _city _vector2int)
            (`BlueprintMapLibrary.Map_Add` _city _vector2int _output_get_3)
            (if (== (`local.Column`) 1)
              (`SceneComponent.K2_SetWorldTransform` (`/Game/Geometry/Meshes/Roads/BaseRoad.DefaultSceneRoot` _current) (`KismetMathLibrary.MakeTransform` (`self.ObjectPos`)) false false)
              (else
                (bind _width (`/Game/Geometry/Meshes/Roads/BaseRoad.GetWidth` _current))
                (bind _output_get_5 (set `self.ObjectPos` (+ (`self.ObjectPos`) (`KismetMathLibrary.MakeVector` 0.0 (`KismetMathLibrary.Conv_IntToDouble` _width)))))
                (`SceneComponent.K2_SetWorldTransform` (`/Game/Geometry/Meshes/Roads/BaseRoad.DefaultSceneRoot` _current) (`KismetMathLibrary.MakeTransform` _output_get_5) false false)))
            (bind _width_2 (`/Game/Geometry/Meshes/Roads/BaseRoad.GetWidth` _current))
            (set `self.ObjectPos` (+ (`self.ObjectPos`) (`KismetMathLibrary.MakeVector` 0.0 (`KismetMathLibrary.Conv_IntToDouble` _width_2))))
            (else
              (return)))
          (else
            (return))))
      (bind _height_2 (`/Game/Geometry/Meshes/Roads/BaseRoad.GetHeight` (`self.Current`)))
      (bind _returnvalue_x (`KismetMathLibrary.BreakVector` (+ (`self.ObjectPos`) (`KismetMathLibrary.MakeVector` (`KismetMathLibrary.Conv_IntToDouble` _height_2)))))
      (set `self.ObjectPos` (`KismetMathLibrary.MakeVector` _returnvalue_x (.y (.location _returnvalue)) (.z (.location _returnvalue)))))
    (`self.PostCreate`)
    (else
      (return))))

(fn `GenerateSeed`
  (bind _returnvalue (`KismetMathLibrary.UtcNow`))
  (`KismetMathLibrary.SetRandomStreamSeed` (`self.CitySeed`) (+ (`KismetMathLibrary.GetMillisecond` _returnvalue) (`KismetMathLibrary.FTrunc` (/ (`KismetMathLibrary.Conv_IntToDouble` (`KismetMathLibrary.GetMinute` _returnvalue)) (`KismetMathLibrary.Conv_IntToDouble` (`KismetMathLibrary.GetSecond` _returnvalue)))))))

(fn `GetRandomPlot`
  (returns (Plot :type "Actor Object Reference"))
  (bind _values (`BlueprintMapLibrary.Map_Values` (`self.City`)))
  (bind _filteredarray (`KismetArrayLibrary.FilterArray` _values "/Game/Geometry/Meshes/Roads/CityBlock_Blueprint.CityBlock_Blueprint_C"))
  (return (`KismetArrayLibrary.Array_RandomFromStream` _filteredarray (`self.CitySeed`))))

(fn `GetRandomRotation`
  (returns (Rotation :type "Rotator Structure"))
  (switch `int` (`KismetMathLibrary.RandomIntegerInRangeFromStream` 0 3 (`self.CitySeed`))
    (:`0`
      (bind _output_get (set `self.Rotator` (struct))))
    (:`1`
      (set `self.Rotator` (struct :`Yaw` 90.0)))
    (:`2`
      (set `self.Rotator` (struct :`Yaw` 180.0)))
    (:`3`
      (set `self.Rotator` (struct :`Yaw` -90.0))))
  (return _output_get))

(fn `MakePowerplant`
  (params (Plot :type "Actor Object Reference"))
  (returns (Final :type "Actor Object Reference"))
  (bind _final (`self.Spawn&AttachRandom` null Plot))
  (return _final))

(fn `MakeResidential`
  (params (Block :type "Actor Object Reference"))
  (returns (Final :type "Actor Object Reference"))
  (switch `int` (`KismetMathLibrary.RandomInteger` 5)
    (:`0`
      (bind _final (`self.Spawn&AttachRandom` null Block)))
    (:`1`
      (`self.Spawn&AttachRandom` null Block))
    (:`2`
      (`self.Spawn&AttachRandom` null)))
  (return _final))

(fn `Populate Plots`
  (locals (PlotClass :type "Actor Class Reference") (SetPlots :type "Array of Actor Object Reference"))
  (bind _plot (`self.GetRandomPlot`))
  (bind _final (`self.MakePowerplant` _plot))
  (bind _values (`BlueprintMapLibrary.Map_Values` (`self.City`)))
  (bind _filteredarray (`KismetArrayLibrary.FilterArray` _values "/Game/Geometry/Meshes/Roads/CityBlock_Blueprint.CityBlock_Blueprint_C"))
  (for _array_element _filteredarray
    (if (not (== _array_element _final))
      (switch `int` (`KismetMathLibrary.RandomIntegerFromStream` 1 (`self.CitySeed`))
        (:`0`
          _)
        (:`1`
          _))
      (`self.MakeResidential` _array_element))))

(fn `PostCreate`
  (`self.SetOffset`)
  (`self.Populate Plots`)
  (`self.SetFinalScale`))

(fn `SetFinalScale`
  (`self.SetActorScale3D` (`self.FinalScale`)))

(fn `SetOffset`
  (bind (_returnvalue_x _returnvalue_y _returnvalue_z) (`KismetMathLibrary.BreakVector` (`self.K2_GetActorLocation`)))
  (bind _city (`self.City`))
  (bind _size_x (break `/Game/Geometry/Meshes/Roads/Vector2Int` (`self.Size`)))
  (bind _city_2 (`self.City`))
  (bind (_size_x_2 _size_y) (break `/Game/Geometry/Meshes/Roads/Vector2Int` (`self.Size`)))
  (bind (_value _returnvalue) (`BlueprintMapLibrary.Map_Find` _city_2 (make `/Game/Geometry/Meshes/Roads/Vector2Int` 1 1)))
  (bind (_value_2 _returnvalue_2) (`BlueprintMapLibrary.Map_Find` _city (make `/Game/Geometry/Meshes/Roads/Vector2Int` 1 1)))
  (bind (_value_3 _returnvalue_3) (`BlueprintMapLibrary.Map_Find` _city (make `/Game/Geometry/Meshes/Roads/Vector2Int` _size_x 1)))
  (bind (_value_4 _returnvalue_4) (`BlueprintMapLibrary.Map_Find` _city_2 (make `/Game/Geometry/Meshes/Roads/Vector2Int` 1 _size_y)))
  (if (and (and _returnvalue _returnvalue_4) (and _returnvalue_2 _returnvalue_3))
    (bind _output_get (set `self.Center` (/ (+ (- (`SceneComponent.K2_GetComponentLocation` (`/Game/Geometry/Meshes/Roads/BaseRoad.Right` _value)) (`SceneComponent.K2_GetComponentLocation` (`/Game/Geometry/Meshes/Roads/BaseRoad.Right` _value_4))) (- (`SceneComponent.K2_GetComponentLocation` (`/Game/Geometry/Meshes/Roads/BaseRoad.Top` _value_2)) (`SceneComponent.K2_GetComponentLocation` (`/Game/Geometry/Meshes/Roads/BaseRoad.Top` _value_3)))) 2.0)))
    (`self.K2_SetActorTransform` (`self.CityOffset`) (`KismetMathLibrary.MakeTransform` (`KismetMathLibrary.MakeVector` (+ _returnvalue_x (.x _output_get)) (+ (.y _output_get) _returnvalue_y) _returnvalue_z)) false false)))

(fn `Spawn&AttachRandom`
  (params (Class :type "Actor Class Reference") (ParentActor :type "Actor Object Reference"))
  (returns (Final :type "Actor Object Reference"))
  (bind _rotation (`self.GetRandomRotation`))
  (bind _returnvalue (`|SpawnActorFromClass` Class (`KismetMathLibrary.MakeTransform` (0.0 0.0 0.0) _rotation) "Undefined" "OverrideRootScale" null null))
  (`self.K2_AttachToActor` _returnvalue ParentActor "None" "KeepRelative" "KeepRelative" "KeepRelative" true)
  (return ParentActor))

(fn `UserConstructionScript`)