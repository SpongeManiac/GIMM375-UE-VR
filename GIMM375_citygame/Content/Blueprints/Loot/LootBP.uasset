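; Loot pickup actor whose LootItem mesh reacts to component hits; SetLoot assigns the mesh and always sets the type to "Battery".
; Hits from player pawn 0 pass the loot to ThirdPersonCharacter_DoNotUse's PickupItem, while a VRPawn match does nothing.
; Any non-player hit destroys the parent actor, as the enemy comparison against BP_ActorToSpawn is computed but unused.
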(event `self.LootItem.OnComponentHit`
  (params (HitComponent :type "PrimitiveComponent Object Reference") (OtherActor :type "Actor Object Reference") (OtherComp :type "PrimitiveComponent Object Reference") (NormalImpulse :type "Vector Structure") (Hit :type "HitResult Structure (by ref)"))
  (`self.LootTouched` OtherActor))

(fn `LootTouched`
  (params (Other :type "Actor Object Reference"))
  (bind _output_get (set `self.IsPlayer` (== Other (`GameplayStatics.GetPlayerPawn` 0))))
  (if _output_get
    (cast `/Game/VRTemplate/Blueprints/VRPawn` Other
      (:`CastFailed`
        (bind _asthird_person_character_do_not_use (cast `/Game/TP/ThirdPersonBP/Blueprints/ThirdPersonCharacter_Current` Other)
          (:`then`
            (`/Game/TP/ThirdPersonBP/Blueprints/ThirdPersonCharacter_Current.PickupItem` _asthird_person_character_do_not_use self))
          (:`CastFailed`
            (`KismetSystemLibrary.PrintString` "Invalid Player")))))
    (else
      (set `self.IsEnemy` (== Other "/Game/BP_ActorToSpawn.BP_ActorToSpawn"))
      (if true
        (`self.K2_DestroyActor` (`self.GetParentActor`))))))

(fn `SetLoot`
  (params (LootMesh :type "StaticMesh Object Reference"))
  (`StaticMeshComponent.SetStaticMesh` (`self.LootItem`) LootMesh)
  (set `self.ItemType` "Battery"))

(fn `UserConstructionScript`)